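; BP_Collectable is a pickup actor that the bird player collects by flying or moving into its sphere collision.
; Shortly after BeginPlay it registers itself with the HUD widget owned by the first player's BP_BirdController.
; When a BP_BirdPlayer overlaps the sphere, it reports the collection to that player's controller HUD widget and then destroys itself.
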(event OnComponentBeginOverlap(SphereCollision)
  (params (OverlappedComponent :type Primitive%20Component%20Object%20Reference) (OtherActor :type Actor%20Object%20Reference) (OtherComp :type Primitive%20Component%20Object%20Reference) (OtherBodyIndex :type Integer) (bFromSweep :type Boolean) (SweepResult :type Hit%20Result%20Structure%20%28by%20ref%29))
  (bind _asbp_bird_player (Utilities|Casting|CastToBP_BirdPlayer OtherActor))
  (bind _asbp_bird_controller (Utilities|Casting|CastToBP_BirdController (Pawn|GetController _asbp_bird_player)))
  (Default|CollectableCollected (Variables|/Game/Blueprints/Controllers/BP_BirdController.BP_BirdController_C|GetHudWidget _asbp_bird_controller) self)
  (Actor|DestroyActor))

(event EventBeginPlay
  (Utilities|FlowControl|Delay 0.1)
  (bind _asbp_bird_controller (Utilities|Casting|CastToBP_BirdController (Game|GetPlayerController 0)))
  (Default|AddCollectable (Variables|/Game/Blueprints/Controllers/BP_BirdController.BP_BirdController_C|GetHudWidget _asbp_bird_controller) self))

(event Collision|EventActorBeginOverlap
  (params (OtherActor :type Actor%20Object%20Reference)))

(event EventTick
  (params (DeltaSeconds :type Float%20%28single-precision%29)))

(fn ConstructionScript)