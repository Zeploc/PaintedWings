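; Checkpoint actor with bobbing leaves and an egg that is shown once the checkpoint is saved.
; BeginPlay stores the floating leaves' starting relative position, and Tick offsets its height by a sine of real time, scaled by bobbing speed and height.
; Tick also polls the IsSaved flag and unhides the egg if it is not visible; the flag is not set within this Blueprint.
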(event EventBeginPlay
  (Variables|Default|SetStartPosition (Variables|/Script/Engine.SceneComponent|GetRelativeLocation (Variables|Default|GetLeavesFloating))))

(event Collision|EventActorBeginOverlap
  (params (OtherActor :type Actor%20Object%20Reference)))

(event EventTick
  (params (DeltaSeconds :type Float%20%28single-precision%29))
  (bind _leavesfloating (Variables|Default|GetLeavesFloating))
  (bind _egg (Variables|Default|GetEgg))
  (bind _relativelocation (Variables|/Script/Engine.SceneComponent|GetRelativeLocation _leavesfloating))
  (bind (_x _y) (Math|Vector|BreakVector _relativelocation))
  (Transformation|SetRelativeLocation _leavesfloating (Math|Vector|MakeVector _x _y (+ (.Z (Math|Vector|BreakVector (Variables|Default|GetStartPosition))) (* (Math|Trig|Sin(Degrees) (* (Utilities|Time|GetRealTimeSeconds) (Variables|Default|GetBobbingSpeed))) (Variables|Default|GetBobbingHeight)))) false false)
  (if (Variables|Default|GetIsSaved)
    (if (not (Rendering|IsVisible _egg))
      (Development|SetHiddeninGame _egg false false))))

(fn ConstructionScript)