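; Tutorial trigger volume that shows a configurable message when the bird player enters its Box.
; Overlap hands the message to the bird controller, passing a flag that requests a tip-only display after the first visit.
; Leaving hides the message through the player's controller.
; Any end overlap also clears PauseOnLand on player controller 0, whichever actor left.
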(event OnComponentBeginOverlap(Box)
  (params (OverlappedComponent :type Primitive%20Component%20Object%20Reference) (OtherActor :type Actor%20Object%20Reference) (OtherComp :type Primitive%20Component%20Object%20Reference) (OtherBodyIndex :type Integer) (bFromSweep :type Boolean) (SweepResult :type Hit%20Result%20Structure%20%28by%20ref%29))
  (bind _asbp_bird_player (Utilities|Casting|CastToBP_BirdPlayer OtherActor))
  (bind _asbp_bird_controller (Utilities|Casting|CastToBP_BirdController (Pawn|GetController _asbp_bird_player)))
  (Default|ShowTutorialMessage _asbp_bird_controller (Variables|Default|GetTutMessage) (Variables|Default|GetBeenToggled))
  (Variables|Default|SetBeenToggled true))

(event OnComponentEndOverlap(Box)
  (params (OverlappedComponent :type Primitive%20Component%20Object%20Reference) (OtherActor :type Actor%20Object%20Reference) (OtherComp :type Primitive%20Component%20Object%20Reference) (OtherBodyIndex :type Integer))
  (CallFunction|HideTutorialMessage OtherActor)
  (bind _asbp_bird_controller (Utilities|Casting|CastToBP_BirdController (Game|GetPlayerController 0)))
  (Variables|/Game/Blueprints/Controllers/BP_BirdController.BP_BirdController_C|SetPauseOnLand _asbp_bird_controller false))

(event EventBeginPlay)

(event Collision|EventActorBeginOverlap
  (params (OtherActor :type Actor%20Object%20Reference)))

(event EventTick
  (params (DeltaSeconds :type Float%20%28single-precision%29)))

(fn ConstructionScript)

(fn HideTutorialMessage
  (params (Object :type Object%20Object%20Reference))
  (bind _asbp_bird_player (Utilities|Casting|CastToBP_BirdPlayer Object))
  (bind _asbp_bird_controller (Utilities|Casting|CastToBP_BirdController (Pawn|GetController _asbp_bird_player)))
  (Default|HideTutorialMessage _asbp_bird_controller))