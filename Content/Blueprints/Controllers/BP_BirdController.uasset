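; Player controller for the bird game that manages HUD, tutorial, pause and end-screen widgets.
; Tutorials show as tips or as messages that pause once the bird lands until Jump; pause toggles only its widget over such messages.
; The end screen freezes the bird, pins its hunger and offers level restart or quit.
; Key presses report gamepad use to the game instance, and UpdateGamepadMode refreshes visible prompts.
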(event EventBeginPlay
  (bind _returnvalue (UserInterface|CreateWidget "/Game/UI/W_HUD.W_HUD_C"))
  (bind _output_get (Variables|Default|SetHudWidget _returnvalue))
  (UserInterface|Viewport|AddtoViewport _output_get 0))

(event EventTick
  (params (DeltaSeconds :type Float%20%28single-precision%29))
  (bind _endscreenwidget (Variables|Default|GetEndScreenWidget))
  (Utilities|FlowControl|Sequence
    (:then_0
      (if (Utilities|IsValid _endscreenwidget)
        (if (Widget|IsVisible _endscreenwidget)
          (bind _asbp_bird_player (Utilities|Casting|CastToBP_BirdPlayer (Game|GetPlayerCharacter 0)))
          (Variables|/Script/PaintedWings.BirdPlayer|SetHungerLevel _asbp_bird_player 1.0))))
    (:then_1
      (if (Variables|Default|GetPauseOnLand)
        (CallFunction|TutPauseGame)))))

(event Input|ActionEvents|InputActionJump
  (params (Key :type Key%20Structure))
  (bind _returnvalue (Game|IsGamePaused))
  (bind _tutwidget (Variables|Default|GetTutWidget))
  (bind _pausewidget (Variables|Default|GetPauseWidget))
  (bind _returnvalue_2 (Widget|IsVisible _tutwidget))
  (:Pressed
    (Utilities|IsValid _tutwidget
      (:Is%20Valid
        (Utilities|IsValid _pausewidget
          (:Is%20Valid
            (if (Math|Boolean|ANDBoolean _returnvalue_2 _returnvalue (not (Widget|IsVisible _pausewidget)))
              (CallFunction|HideTutorialMessage :!label _label)
              (Game|SetGamePaused false)
              (bind _asbp_bird_player (Utilities|Casting|CastToBP_BirdPlayer (Game|Player|GetPlayerPawn 0)))
              (Variables|/Script/PaintedWings.BirdPlayer|SetbLookAtNext _asbp_bird_player false)))
          (:Is%20Not%20Valid
            (if (and _returnvalue_2 _returnvalue)
              (goto _label))))))))

(event Input|GamepadEvents|GamepadSpecialRight
  (params (Key :type Key%20Structure))
  (:Pressed
    (Utilities|IsValid (Variables|Default|GetEndScreenWidget)
      (:Is%20Valid
        (Game|OpenLevel(byName) "TestLevel"))
      (:Is%20Not%20Valid
        (CallFunction|TogglePause)))))

(event Input|KeyboardEvents|Enter
  (params (Key :type Key%20Structure))
  (:Pressed
    (Utilities|IsValid (Variables|Default|GetEndScreenWidget)
      (:Is%20Valid
        (Game|OpenLevel(byName) "TestLevel"))
      (:Is%20Not%20Valid
        (CallFunction|TogglePause)))))

(event Input|KeyboardEvents|Escape
  (params (Key :type Key%20Structure))
  (bind _endscreenwidget (Variables|Default|GetEndScreenWidget))
  (:Pressed
    (if (Utilities|IsValid _endscreenwidget)
      (if (Widget|IsVisible _endscreenwidget)
        (Game|QuitGame 0 "Quit")))))

(event Input|GamepadEvents|GamepadSpecialLeft
  (params (Key :type Key%20Structure))
  (bind _endscreenwidget (Variables|Default|GetEndScreenWidget))
  (:Pressed
    (if (Utilities|IsValid _endscreenwidget)
      (if (Widget|IsVisible _endscreenwidget)
        (Game|QuitGame 0 "Quit")))))

(event Input|KeyboardEvents|AnyKey
  (params (Key :type Key%20Structure))
  (:Pressed
    (bind _asgi (Utilities|Casting|CastToGI (Game|GetGameInstance)))
    (Default|SwitchUsingGamepad _asgi (Class|KismetInputLibrary|KeyIsGamepadKey Key))))

(fn ConstructionScript)

(fn EndScreen
  (bind _returnvalue (Game|GetPlayerCharacter 0))
  (bind _hudwidget (Variables|Default|GetHudWidget))
  (Utilities|IsValid _hudwidget
    (:Is%20Valid
      (Widget|SetVisibility _hudwidget "Hidden"))
    (:Is%20Not%20Valid
      _))
  (bind _returnvalue_2 (UserInterface|CreateWidget "/Game/UI/W_EndScreen.W_EndScreen_C"))
  (bind _output_get (Variables|Default|SetEndScreenWidget _returnvalue_2))
  (UserInterface|Viewport|AddtoViewport _output_get 0)
  (Input|DisableInput _returnvalue self)
  (Pawn|Components|CharacterMovement|DisableMovement (Variables|/Script/Engine.Character|GetCharacterMovement _returnvalue)))

(fn ShowTutorialMessage
  (params (Message :type Text) (TipOnly :type Boolean) (Input :type GameInput%20Enum :default "NewEnumerator0"))
  (bind _isactive (CallFunction|IsTutorialActive))
  (if (not _isactive)
    (if TipOnly
      (Utilities|IsValid (Variables|Default|GetTutWidgetTip)
        (:Is%20Valid
          _)
        (:Is%20Not%20Valid
          (bind _returnvalue (UserInterface|CreateWidget "/Game/UI/W_Tut_Tip.W_Tut_Tip_C"))
          (bind _output_get (Variables|Default|SetTutWidgetTip _returnvalue))
          (UserInterface|Viewport|AddtoViewport _output_get 0)))
      (Widget|SetVisibility (Variables|Default|GetTutWidgetTip) "Visible")
      (Rendering|Components|TextRender|SetText (Variables|/Game/UI/W_Tut_Tip.W_Tut_Tip_C|GetTutMessage (Variables|Default|GetTutWidgetTip)) Message)
      (Default|SetButton (Variables|Default|GetTutWidgetTip) Input)
      (else
        (Utilities|IsValid (Variables|Default|GetTutWidget)
          (:Is%20Valid
            _)
          (:Is%20Not%20Valid
            (bind _returnvalue_2 (UserInterface|CreateWidget "/Game/UI/W_Tut.W_Tut_C"))
            (bind _output_get_2 (Variables|Default|SetTutWidget _returnvalue_2))
            (UserInterface|Viewport|AddtoViewport _output_get_2 0)))
        (Widget|SetVisibility (Variables|Default|GetTutWidget) "Visible")
        (Rendering|Components|TextRender|SetText (Variables|/Game/UI/W_Tut.W_Tut_C|GetTutMessage (Variables|Default|GetTutWidget)) Message)
        (Default|SetButton (Variables|Default|GetTutWidget) Input)
        (Variables|Default|SetPauseOnLand true)))))

(fn HideTutorialMessage
  (bind _tutwidget (Variables|Default|GetTutWidget))
  (bind _tutwidgettip (Variables|Default|GetTutWidgetTip))
  (Utilities|FlowControl|Sequence
    (:then_0
      (Utilities|IsValid _tutwidget
        (:Is%20Valid
          (Widget|SetVisibility _tutwidget "Hidden"))))
    (:then_1
      (Utilities|IsValid _tutwidgettip
        (:Is%20Valid
          (Widget|SetVisibility _tutwidgettip "Hidden"))))))

(fn TutPauseGame
  (bind _tutwidget (Variables|Default|GetTutWidget))
  (if (not (AI|Components|NavMovement|IsFalling (Variables|/Script/Engine.Character|GetCharacterMovement (Game|GetPlayerCharacter 0))))
    (Utilities|IsValid _tutwidget
      (:Is%20Valid
        (if (Widget|IsVisible _tutwidget)
          (Game|SetGamePaused true)
          (Variables|Default|SetPauseOnLand false))))))

(fn IsTutorialActive
  (bind _tutwidget (Variables|Default|GetTutWidget))
  (bind _tutwidgettip (Variables|Default|GetTutWidgetTip))
  (Utilities|IsValid _tutwidget
    (:Is%20Valid
      (if (Widget|IsVisible _tutwidget)
        (return true)
        (else
          _)))
    (:Is%20Not%20Valid
      _))
  (Utilities|IsValid _tutwidgettip
    (:Is%20Valid
      (if (Widget|IsVisible _tutwidgettip)
        (return true)
        (else
          _)))
    (:Is%20Not%20Valid
      _))
  (return false))

(fn SetPause
  (params (IsPause :type Boolean) (OnlyWidget :type Boolean))
  (if OnlyWidget
    _
    (else
      (Game|SetGamePaused IsPause)))
  (if IsPause
    (Utilities|IsValid (Variables|Default|GetPauseWidget)
      (:Is%20Valid
        (Widget|SetVisibility (Variables|Default|GetPauseWidget) "Visible"))
      (:Is%20Not%20Valid
        (bind _returnvalue (UserInterface|CreateWidget "/Game/UI/W_PauseScreen.W_PauseScreen_C"))
        (bind _output_get (Variables|Default|SetPauseWidget _returnvalue))
        (UserInterface|Viewport|AddtoViewport _output_get 1)))
    (Default|SetGamepadButton (Variables|Default|GetPauseWidget))
    (else
      (bind _asbp_bird_player (Utilities|Casting|CastToBP_BirdPlayer (Game|Player|GetPlayerPawn 0)))
      (Variables|/Script/PaintedWings.BirdPlayer|SetbLookAtNext _asbp_bird_player false)
      (Utilities|IsValid (Variables|Default|GetPauseWidget)
        (:Is%20Valid
          (Widget|SetVisibility (Variables|Default|GetPauseWidget) "Hidden"))))))

(fn TogglePause
  (bind _pausewidget (Variables|Default|GetPauseWidget))
  (bind _tutwidget (Variables|Default|GetTutWidget))
  (Utilities|IsValid _tutwidget
    (:Is%20Valid
      (if (Widget|IsVisible _tutwidget)
        (Utilities|IsValid _pausewidget
          (:Is%20Valid
            (if (Widget|IsVisible _pausewidget)
              (CallFunction|SetPause false true)
              (else
                (CallFunction|SetPause true true :!label _label))))
          (:Is%20Not%20Valid
            (goto _label)))
        (else
          (CallFunction|SetPause (not (Game|IsGamePaused)) false :!label _label_2))))
    (:Is%20Not%20Valid
      (goto _label_2))))

(fn SetCurrentTutorialGamepadMode
  (bind _tutwidget (Variables|Default|GetTutWidget))
  (bind _tutwidgettip (Variables|Default|GetTutWidgetTip))
  (Utilities|IsValid _tutwidget
    (:Is%20Valid
      (if (Widget|IsVisible _tutwidget)
        (Default|UpdateInputType _tutwidget)
        (else
          (Utilities|IsValid _tutwidgettip :!label _label
            (:Is%20Valid
              (if (Widget|IsVisible _tutwidgettip)
                (Default|UpdateInputType _tutwidgettip)))))))
    (:Is%20Not%20Valid
      (goto _label))))

(fn UpdateGamepadMode
  (CallFunction|SetCurrentTutorialGamepadMode)
  (CallFunction|SetPauseGamepadMode))

(fn SetPauseGamepadMode
  (bind _pausewidget (Variables|Default|GetPauseWidget))
  (Utilities|IsValid _pausewidget
    (:Is%20Valid
      (if (Widget|IsVisible _pausewidget)
        (Default|SetGamepadButton _pausewidget)))))