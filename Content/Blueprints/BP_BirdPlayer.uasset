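; BP_BirdPlayer is the bird player Blueprint, handling per-frame movement limits for gliding and vine climbing.
; While gliding, Tick clamps downward velocity to the glide fall-speed cap, leaving horizontal motion untouched.
; Otherwise, while climbing vines with gravity scale above zero, Tick zeroes all movement velocity.
; The glide and climb states are only read here, and BeginPlay, overlap and construction logic are empty.
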(event EventBeginPlay)

(event Collision|EventActorBeginOverlap
  (params (OtherActor :type Actor%20Object%20Reference)))

(event EventTick
  (params (DeltaSeconds :type Float%20%28single-precision%29))
  (bind _charactermovement (Variables|Character|GetCharacterMovement))
  (bind _glidecapfallspeed (Variables|Default|GetGlideCapFallSpeed))
  (bind _returnvalue (* _glidecapfallspeed -1.0))
  (if (Variables|Default|GetbIsGliding)
    (if (< (.Z (Math|Vector|BreakVector (Transformation|GetVelocity))) _returnvalue)
      (Variables|/Script/Engine.MovementComponent|SetVelocity _charactermovement (Math|Vector|MakeVector (.X (Math|Vector|BreakVector (Variables|/Script/Engine.MovementComponent|GetVelocity _charactermovement))) (.Y (Math|Vector|BreakVector (Variables|/Script/Engine.MovementComponent|GetVelocity _charactermovement))) _returnvalue)))
    (elif (Variables|Default|GetbClimbingVines)
      (if (> (Variables|/Script/Engine.CharacterMovementComponent|GetGravityScale _charactermovement) 0.0)
        (Variables|/Script/Engine.MovementComponent|SetVelocity _charactermovement "0, 0, 0")))))

(fn ConstructionScript)