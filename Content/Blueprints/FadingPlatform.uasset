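; FadingPlatform is a platform actor that repeatedly fades out and back in, losing collision while gone.
; BeginPlay creates a dynamic material for its mesh and seeds a start offset countdown.
; After that offset, Tick steps the Opacity parameter by a fixed per-frame increment, holding at full opacity for SolidTime.
; At zero opacity it disables collision, waits on a short Delay, then restores collision and fades in.
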(event EventBeginPlay
  (bind _staticmesh (Variables|Default|GetStaticMesh))
  (Variables|Default|SetCurrentOffsetDelay (Variables|PlatformSettings|GetStartOffsetDelay))
  (bind _returnvalue (Rendering|Material|CreateDynamicMaterialInstance _staticmesh 0 (Rendering|Material|GetMaterial _staticmesh 0) "None" :!class /Script/Engine.PrimitiveComponent))
  (Variables|Default|SetDynMat _returnvalue)
  (Rendering|Material|SetScalarParameterValue (Variables|Default|GetDynMat) "Opacity" (Variables|Default|GetOpacity) :!class /Script/Engine.MaterialInstanceDynamic)
  (Rendering|Material|SetMaterial _staticmesh 0 (Variables|Default|GetDynMat)))

(event Collision|EventActorBeginOverlap
  (params (OtherActor :type Actor%20Object%20Reference)))

(event EventTick
  (params (DeltaSeconds :type Float%20%28single-precision%29))
  (bind _incrementer (Variables|Default|GetIncrementer))
  (if (> (Variables|Default|GetCurrentOffsetDelay) 0.0)
    (Variables|Default|SetCurrentOffsetDelay (- (Variables|Default|GetCurrentOffsetDelay) DeltaSeconds))
    (else
      (Rendering|Material|SetMaterial (Variables|Default|GetStaticMesh) 0 (Variables|Default|GetDynMat))
      (if (> (Variables|Default|GetCurrentSolidTime) 0.0)
        (Variables|Default|SetCurrentSolidTime (- (Variables|Default|GetCurrentSolidTime) DeltaSeconds))
        (else
          (if (Variables|Default|GetbGone)
            (Collision|SetCollisionEnabled (Variables|Default|GetStaticMesh) "NoCollision")
            (else
              (Collision|SetCollisionEnabled (Variables|Default|GetStaticMesh) "QueryAndPhysics")))
          (if (Variables|Default|GetbGone)
            (Utilities|FlowControl|Delay 1.0)
            (Variables|Default|SetbGone false)
            (Variables|Default|SetIncreaing true)
            (else
              (if (Variables|Default|GetIncreaing)
                (Variables|Default|SetOpacity (+ (Variables|Default|GetOpacity) _incrementer))
                (else
                  (Variables|Default|SetOpacity (- (Variables|Default|GetOpacity) _incrementer))))
              (Rendering|Material|SetScalarParameterValue (Variables|Default|GetDynMat) "Opacity" (Variables|Default|GetOpacity) :!class /Script/Engine.MaterialInstanceDynamic)
              (if (>= (Variables|Default|GetOpacity) 1.0)
                (Variables|Default|SetIncreaing false)
                (Variables|Default|SetCurrentSolidTime (Variables|PlatformSettings|GetSolidTime))
                (elif (<= (Variables|Default|GetOpacity) 0.0)
                  (Variables|Default|SetOpacity 0.0)
                  (Variables|Default|SetbGone true))))))))))

(fn ConstructionScript)