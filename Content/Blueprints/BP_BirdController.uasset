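; Player controller for the bird game that manages the UI flow from start menu through play to end screen.
; BeginPlay shows the menu with the bird hidden and frozen; Enter swaps to the HUD, restores control and refills hunger.
; EndScreen freezes the player again, Tick then pins hunger at full, and Enter reloads TestLevel.
; It also exposes functions to show and hide a lazily created tutorial message widget.
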(event EventBeginPlay
  (bind _returnvalue (Game|GetPlayerCharacter 0))
  (bind _returnvalue_2 (UserInterface|CreateWidget "/Game/UI/W_Menu.W_Menu_C"))
  (bind _output_get (Variables|Default|SetMenuWidget _returnvalue_2))
  (UserInterface|Viewport|AddtoViewport _output_get 0)
  (Input|DisableInput _returnvalue self)
  (Pawn|Components|CharacterMovement|DisableMovement (Variables|/Script/Engine.Character|GetCharacterMovement _returnvalue))
  (bind _asbp_bird_player (Utilities|Casting|CastToBP_BirdPlayer _returnvalue))
  (Rendering|SetVisibility (Variables|/Script/Engine.Character|GetMesh _asbp_bird_player) false false))

(event EventTick
  (params (DeltaSeconds :type Float%20%28single-precision%29))
  (Utilities|IsValid (Variables|Default|GetEndScreenWidget)
    (:Is%20Valid
      (bind _asbp_bird_player (Utilities|Casting|CastToBP_BirdPlayer (Game|GetPlayerCharacter 0)))
      (Variables|/Script/PaintedWings.BirdPlayer|SetHungerLevel _asbp_bird_player 1.0))))

(event Input|KeyboardEvents|Enter
  (params (Key :type Key%20Structure))
  (bind _returnvalue (Game|GetPlayerCharacter 0))
  (:Pressed
    (if (Widget|IsVisible (Variables|Default|GetMenuWidget))
      (Widget|SetVisibility (Variables|Default|GetMenuWidget) "Hidden")
      (bind _returnvalue_2 (UserInterface|CreateWidget "/Game/UI/W_HUD.W_HUD_C"))
      (bind _output_get (Variables|Default|SetHudWidget _returnvalue_2))
      (UserInterface|Viewport|AddtoViewport _output_get 0)
      (Input|EnableInput _returnvalue self)
      (Pawn|Components|CharacterMovement|SetMovementMode (Variables|/Script/Engine.Character|GetCharacterMovement _returnvalue) "MOVE_Walking" 0)
      (bind _asbp_bird_player (Utilities|Casting|CastToBP_BirdPlayer _returnvalue))
      (Variables|/Script/PaintedWings.BirdPlayer|SetHungerLevel _asbp_bird_player 1.0)
      (Rendering|SetVisibility (Variables|/Script/Engine.Character|GetMesh _asbp_bird_player) true false)
      (else
        (Utilities|IsValid (Variables|Default|GetEndScreenWidget)
          (:Is%20Valid
            (Game|OpenLevel(byName) "TestLevel")))))))

(fn ConstructionScript)

(fn EndScreen
  (bind _returnvalue (Game|GetPlayerCharacter 0))
  (bind _hudwidget (Variables|Default|GetHudWidget))
  (Utilities|IsValid _hudwidget
    (:Is%20Valid
      (Widget|SetVisibility _hudwidget "Hidden"))
    (:Is%20Not%20Valid
      _))
  (bind _returnvalue_2 (UserInterface|CreateWidget "/Game/UI/W_EndScreen.W_EndScreen_C"))
  (bind _output_get (Variables|Default|SetEndScreenWidget _returnvalue_2))
  (UserInterface|Viewport|AddtoViewport _output_get 0)
  (Input|DisableInput _returnvalue self)
  (Pawn|Components|CharacterMovement|DisableMovement (Variables|/Script/Engine.Character|GetCharacterMovement _returnvalue)))

(fn ShowTutorialMessage
  (params (Message :type Text))
  (Utilities|IsValid (Variables|Default|GetTutWidget)
    (:Is%20Valid
      _)
    (:Is%20Not%20Valid
      (bind _returnvalue (UserInterface|CreateWidget "/Game/UI/W_Tut.W_Tut_C"))
      (bind _output_get (Variables|Default|SetTutWidget _returnvalue))
      (UserInterface|Viewport|AddtoViewport _output_get 0)))
  (Widget|SetVisibility (Variables|Default|GetTutWidget) "Visible")
  (Rendering|Components|TextRender|SetText (Variables|/Game/UI/W_Tut.W_Tut_C|GetTutMessage (Variables|Default|GetTutWidget)) Message))

(fn HideTutorialMessage
  (bind _tutwidget (Variables|Default|GetTutWidget))
  (Utilities|IsValid _tutwidget
    (:Is%20Valid
      (Widget|SetVisibility _tutwidget "Hidden"))))