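; BendyFlower is a flower actor that computes a 2D bend vector in response to the player bird touching it.
; Overlap events on the Check component store the BP_BirdPlayer and toggle Overlapping.
; While overlapping, Tick accumulates the bird's scale-normalized XY offset into Direction with Y flipped; otherwise it steps Direction back toward zero at ReturnSpeed.
; Direction is only computed here; nothing in these graphs applies it visually.
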(event OnComponentBeginOverlap(Check)
  (params (OverlappedComponent :type Primitive%20Component%20Object%20Reference) (OtherActor :type Actor%20Object%20Reference) (OtherComp :type Primitive%20Component%20Object%20Reference) (OtherBodyIndex :type Integer) (bFromSweep :type Boolean) (SweepResult :type Hit%20Result%20Structure%20%28by%20ref%29))
  (bind _asbp_bird_player (Utilities|Casting|CastToBP_BirdPlayer OtherActor))
  (Variables|Default|SetBirdRef _asbp_bird_player)
  (Variables|Default|SetOverlapping true))

(event OnComponentEndOverlap(Check)
  (params (OverlappedComponent :type Primitive%20Component%20Object%20Reference) (OtherActor :type Actor%20Object%20Reference) (OtherComp :type Primitive%20Component%20Object%20Reference) (OtherBodyIndex :type Integer))
  (Utilities|Casting|CastToBP_BirdPlayer OtherActor)
  (Variables|Default|SetOverlapping false))

(event EventBeginPlay)

(event Collision|EventActorBeginOverlap
  (params (OtherActor :type Actor%20Object%20Reference)))

(event EventTick
  (params (DeltaSeconds :type Float%20%28single-precision%29))
  (bind _check (Variables|Default|GetCheck))
  (bind _birdref (Variables|Default|GetBirdRef))
  (bind _check_2 (Variables|Default|GetCheck))
  (bind _returnvalue (Transformation|GetWorldLocation _check))
  (bind _returnvalue_2 (Transformation|GetWorldScale _check_2))
  (bind _returnvalue_3 (Transformation|GetActorLocation _birdref))
  (bind _returnvalue_4 (- _returnvalue_3 _returnvalue))
  (if (Variables|Default|GetOverlapping)
    (Variables|Default|SetDirection (Math|Vector|MakeVector (+ (.x (Variables|Default|GetDirection)) (/ (.x _returnvalue_4) (* (.x _returnvalue_2) 4e+01))) (+ (.y (Variables|Default|GetDirection)) (* (/ (.y _returnvalue_4) (* (.y _returnvalue_2) 4e+01)) -1.0)) 0.0))
    (else
      (Variables|Default|SetDirection (+ (Variables|Default|GetDirection) (Math|Vector|MakeVector (.x (* (Math|Vector|Normalize (* (Variables|Default|GetDirection) -1.0)) (* (Variables|Default|GetReturnSpeed) DeltaSeconds))) (.y (* (Math|Vector|Normalize (* (Variables|Default|GetDirection) -1.0)) (* (Variables|Default|GetReturnSpeed) DeltaSeconds))) 0.0))))))

(fn ConstructionScript)