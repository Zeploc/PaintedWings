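; Camera actor that switches the player's view to a camera that tracks BP_BirdPlayer, going by its name for a trunk area.
; Box overlap blends the view to this actor and back to the bird on exit; EnableByDefault also activates it at BeginPlay.
; Tick keeps the camera's XY, follows the bird's height plus AboveHeight and aims at it.
; Tick also re-requests this view target every frame, regardless of overlap.
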(event OnComponentBeginOverlap(Box)
  (params (OverlappedComponent :type Primitive%20Component%20Object%20Reference) (OtherActor :type Actor%20Object%20Reference) (OtherComp :type Primitive%20Component%20Object%20Reference) (OtherBodyIndex :type Integer) (bFromSweep :type Boolean) (SweepResult :type Hit%20Result%20Structure%20%28by%20ref%29))
  (bind _asbp_bird_player (Utilities|Casting|CastToBP_BirdPlayer OtherActor))
  (bind _output_get (Variables|Default|SetPlayerRef _asbp_bird_player))
  (bind _asplayer_controller (Utilities|Casting|CastToPlayerController (Pawn|GetController _output_get)))
  (Game|Player|SetViewTargetwithBlend _asplayer_controller self 0.5 "VTBlend_Linear" 0.0 false))

(event OnComponentEndOverlap(Box)
  (params (OverlappedComponent :type Primitive%20Component%20Object%20Reference) (OtherActor :type Actor%20Object%20Reference) (OtherComp :type Primitive%20Component%20Object%20Reference) (OtherBodyIndex :type Integer))
  (bind _playerref (Variables|Default|GetPlayerRef))
  (Utilities|Casting|CastToBP_BirdPlayer OtherActor)
  (bind _asplayer_controller (Utilities|Casting|CastToPlayerController (Pawn|GetController _playerref)))
  (Game|Player|SetViewTargetwithBlend _asplayer_controller _playerref 0.2 "VTBlend_EaseIn" 0.0 false))

(event EventBeginPlay
  (if (Variables|Default|GetEnableByDefault)
    (bind _asbp_bird_player (Utilities|Casting|CastToBP_BirdPlayer (Game|GetPlayerCharacter 0)))
    (bind _output_get (Variables|Default|SetPlayerRef _asbp_bird_player))
    (bind _asplayer_controller (Utilities|Casting|CastToPlayerController (Pawn|GetController _output_get)))
    (Game|Player|SetViewTargetwithBlend _asplayer_controller self 0.5 "VTBlend_Linear" 0.0 false)))

(event Collision|EventActorBeginOverlap
  (params (OtherActor :type Actor%20Object%20Reference)))

(event EventTick
  (params (DeltaSeconds :type Float%20%28single-precision%29))
  (bind _camera (Variables|Default|GetCamera))
  (bind _returnvalue (Transformation|GetWorldLocation _camera))
  (bind (_x _y) (Math|Vector|BreakVector _returnvalue))
  (Utilities|IsValid (Variables|Default|GetPlayerRef)
    (:Is%20Valid
      _)
    (:Is%20Not%20Valid
      (bind _outactors (Actor|GetAllActorsOfClass "/Game/Blueprints/BP_BirdPlayer.BP_BirdPlayer_C"))
      (Variables|Default|SetPlayerRef (Utilities|Array|Get(acopy) _outactors))))
  (Game|Player|SetViewTargetwithBlend (Game|GetPlayerController 0) self 0.5 "VTBlend_Linear" 0.0 false)
  (Transformation|SetWorldRotation _camera (Math|Rotator|FindLookatRotation _returnvalue (Transformation|GetActorLocation (Variables|Default|GetPlayerRef))) false false)
  (Transformation|SetWorldLocation _camera (Math|Vector|MakeVector _x _y (+ (.Z (Math|Vector|BreakVector (Transformation|GetActorLocation (Variables|Default|GetPlayerRef)))) (Variables|Default|GetAboveHeight))) false false))

(fn ConstructionScript)