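; Tube slide actor that propels the bird player along a set direction while it is inside a cylinder volume.
; On overlap it stores the bird, turns it to face the Direction component's forward vector and launches it at LaunchSize speed with velocity override.
; Tick repeats the launch and keeps the bird's dashing flag set until overlap ends, which clears it.
; BeginPlay sets a short particle lifetime.
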(event OnComponentBeginOverlap(Cylinder)
  (params (OverlappedComponent :type Primitive%20Component%20Object%20Reference) (OtherActor :type Actor%20Object%20Reference) (OtherComp :type Primitive%20Component%20Object%20Reference) (OtherBodyIndex :type Integer) (bFromSweep :type Boolean) (SweepResult :type Hit%20Result%20Structure%20%28by%20ref%29))
  (bind _asbp_bird_player (Utilities|Casting|CastToBP_BirdPlayer OtherActor))
  (bind _output_get (Variables|Default|SetBirdRef _asbp_bird_player))
  (Character|LaunchCharacter _asbp_bird_player (* (Math|Vector|GetForwardVector (Variables|Default|GetDirection)) (Variables|Default|GetLaunchSize)) true true)
  (Variables|Default|SetOverlapping true)
  (Variables|/Script/PaintedWings.BirdPlayer|SetIsDashing _output_get true)
  (Transformation|SetActorRotation (Variables|Default|GetBirdRef) (Math|Conversions|RotationFromXVector (Math|Vector|GetForwardVector (Variables|Default|GetDirection)))))

(event OnComponentEndOverlap(Cylinder)
  (params (OverlappedComponent :type Primitive%20Component%20Object%20Reference) (OtherActor :type Actor%20Object%20Reference) (OtherComp :type Primitive%20Component%20Object%20Reference) (OtherBodyIndex :type Integer))
  (bind _asbp_bird_player (Utilities|Casting|CastToBP_BirdPlayer OtherActor))
  (Variables|Default|SetOverlapping false)
  (Variables|/Script/PaintedWings.BirdPlayer|SetIsDashing _asbp_bird_player false))

(event EventBeginPlay
  (Effects|Components|ParticleSystem|SetFloatParameter (Variables|Default|GetParticleSystem) "Lifetime" 0.1))

(event Collision|EventActorBeginOverlap
  (params (OtherActor :type Actor%20Object%20Reference)))

(event EventTick
  (params (DeltaSeconds :type Float%20%28single-precision%29))
  (bind _birdref (Variables|Default|GetBirdRef))
  (if (Variables|Default|GetOverlapping)
    (Utilities|IsValid _birdref
      (:Is%20Valid
        (Character|LaunchCharacter _birdref (* (Math|Vector|GetForwardVector (Variables|Default|GetDirection)) (Variables|Default|GetLaunchSize)) true true)
        (Variables|/Script/PaintedWings.BirdPlayer|SetIsDashing _birdref true)))))

(fn ConstructionScript)