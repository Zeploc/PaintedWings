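; Timed flower trap that cycles between open, with its cylinder blocking pawns, and closed, with that collision ignored.
; Function-name timers chain close, collision off, reopen and collision on, starting after an optional initial delay and repeating at random intervals.
; When collision drops, player 0 within the horizontal kickoff distance is launched away from the cylinder, or in a random horizontal direction if near its center.
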(event EventBeginPlay
  (bind _initialdelay (Variables|Default|GetInitialDelay))
  (if (<= _initialdelay 0.0)
    (CallFunction|PlayTrap)
    (else
      (Utilities|Time|SetTimerbyFunctionName 0 "PlayTrap" _initialdelay))))

(event Collision|EventActorBeginOverlap
  (params (OtherActor :type Actor%20Object%20Reference)))

(event EventTick
  (params (DeltaSeconds :type Float%20%28single-precision%29)))

(fn ConstructionScript)

(fn PlayTrap
  (Utilities|Time|ClearandInvalidateTimerbyHandle (Variables|Default|GetEnableCollisionHandle))
  (Components|Animation|PlayAnimation (Variables|Default|GetSkeletalMesh) "/Game/Meshes/FlowerCloseAnim.FlowerCloseAnim" false)
  (Utilities|Time|SetTimerbyFunctionName 0 "OpenTrap" (+ (Variables|Default|GetCloseHoldTime) 0.5))
  (Utilities|Time|SetTimerbyFunctionName 0 "DisableCollision" 0.5))

(fn DisableCollision
  (bind _returnvalue (Game|GetPlayerCharacter 0))
  (bind _cylinder (Variables|Default|GetCylinder))
  (bind _returnvalue_2 (Transformation|GetWorldLocation _cylinder))
  (bind _returnvalue_3 (Transformation|GetActorLocation _returnvalue))
  (bind _returnvalue_4 (- _returnvalue_3 _returnvalue_2))
  (bind (_x _y) (Math|Vector|BreakVector _returnvalue_4))
  (bind _returnvalue_5 (Math|Vector|MakeVector _x _y 0.0))
  (bind _returnvalue_6 (Math|Vector|VectorLength _returnvalue_5))
  (Collision|SetCollisionResponsetoChannel (Variables|Default|GetCylinder) "ECC_Pawn" "ECR_Ignore")
  (if (< _returnvalue_6 (Variables|Default|GetKickoffDistance))
    (if (> _returnvalue_6 5e+01)
      (Character|LaunchCharacter _returnvalue (* _returnvalue_5 4.0) false false)
      (else
        (Character|LaunchCharacter _returnvalue (* (Math|Vector|MakeVector (Math|Random|RandomFloatinRange -1.0 1.0) (Math|Random|RandomFloatinRange -1.0 1.0) 0.0) 3e+02) false false)))))

(fn EnableCollision
  (Collision|SetCollisionResponsetoChannel (Variables|Default|GetCylinder) "ECC_Pawn" "ECR_Block")
  (Utilities|Time|SetTimerbyFunctionName 0 "PlayTrap" (Math|Random|RandomFloatinRange (Variables|Default|GetMinRan) (Variables|Default|GetMaxRand))))

(fn OpenTrap
  (Utilities|Time|ClearandInvalidateTimerbyHandle (Variables|Default|GetEnableCollisionHandle))
  (Components|Animation|PlayAnimation (Variables|Default|GetSkeletalMesh) "/Game/Meshes/FlowerOpenAnim.FlowerOpenAnim" false)
  (bind _returnvalue (Utilities|Time|SetTimerbyFunctionName 0 "EnableCollision" 0.5))
  (Variables|Default|SetEnableCollisionHandle _returnvalue))